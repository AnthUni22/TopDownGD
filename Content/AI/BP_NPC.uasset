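; BP_NPC is an AI character with health that is destroyed when damage drains it to zero.
; On BeginPlay it casts its mesh's anim instance to ABP_Alien and stores the reference.
; AnyDamage subtracts incoming damage from Health, while StartShooting is an empty event and the Weapon variable is unused.
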(event `self.ReceiveBeginPlay`
  (bind _asabp_alien (cast `/Game/AI/ABP_Alien` (`SkeletalMeshComponent.GetAnimInstance` (`self.Mesh`))))
  (set `self.AnimInstance` _asabp_alien))

(event `StartShooting`)

(event `self.ReceiveAnyDamage`
  (params (Damage :type "Float (single-precision)") (DamageType :type "DamageType Object Reference") (InstigatedBy :type "Controller Object Reference") (DamageCauser :type "Actor Object Reference"))
  ;[1 1 1] Any Damage
  (set `self.Health` (- (`self.Health`) Damage))
  (if (<= (`self.Health`) 0.0)
    (`self.K2_DestroyActor`)))

(fn `UserConstructionScript`)
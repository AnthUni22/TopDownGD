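; BP_AI is an AI character with health that dies when damage reduces it to zero.
; AnyDamage subtracts from Health, then a DoOnce plays the death animation, disables movement and destroys the actor five seconds later.
; A shooting chain that spawns BP_Bullet at BulletSpawnPoint, throttled by a ShootDelay flag and one-second delay, is present but unconnected, so it never runs.
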(event `self.ReceiveBeginPlay`
  (set `self.Health` (`self.Health`)))

(event `self.ReceiveAnyDamage`
  (params (Damage :type "Float (single-precision)") (DamageType :type "DamageType Object Reference") (InstigatedBy :type "Controller Object Reference") (DamageCauser :type "Actor Object Reference"))
  ;[1 1 1] Event Damage AG
  (set `self.Health` (- (`self.Health`) Damage))
  (if (<= (`self.Health`) 0.0)
    (`/Engine/EditorBlueprintResources/StandardMacros.DoOnce` false
      (:`Completed`
        (`SkeletalMeshComponent.PlayAnimation` (`self.Mesh`) "/Game/AI/AI_New/Animations/Death.Death" false)
        (`CharacterMovementComponent.DisableMovement` (`self.CharacterMovement`))
        (`KismetSystemLibrary.Delay` 5.0)
        (`self.K2_DestroyActor`)))))

(fn `UserConstructionScript`)
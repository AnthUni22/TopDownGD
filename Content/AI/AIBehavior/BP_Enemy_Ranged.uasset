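; BP_Enemy_Ranged is a ranged enemy that fires bullets, extending a parent enemy Blueprint.
; On BeginPlay it assigns BT_Ranged to its BP_AIControllerBase and injects it into the running behavior tree as a dynamic subtree under the SubAttack tag.
; The Shoot event spawns a BP_Bullet at BulletSpawnPoint's location and rotation.
; DeathAnimation plays the non-looping Death animation on the mesh.
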(event `self.ReceiveBeginPlay`
  (`parent.ReceiveBeginPlay`)
  (bind _asbp_aicontroller_base (cast `/Game/AI/AIBehavior/BP_AIControllerBase` (`self.GetController`)))
  (set `/Game/AI/AIBehavior/BP_AIControllerBase.BT_AttackAsset` "/Game/AI/AIBehavior/BT/BT_Ranged.BT_Ranged" _asbp_aicontroller_base)
  (bind _asbehavior_tree_component (cast `BehaviorTreeComponent` (`AIController.BrainComponent` (`AIBlueprintHelperLibrary.GetAIController` self))))
  (`BehaviorTreeComponent.SetDynamicSubtree` _asbehavior_tree_component (struct :`TagName` "SubAttack") "/Game/AI/AIBehavior/BT/BT_Ranged.BT_Ranged"))

(event `Shoot`
  (bind (_returnvalue_location _returnvalue_rotation) (`KismetMathLibrary.BreakTransform` (`SceneComponent.K2_GetComponentToWorld` (`self.BulletSpawnPoint`))))
  (`|SpawnActorFromClass` "/Game/AI/RangedAssets/BP_Bullet.BP_Bullet_C" (`KismetMathLibrary.MakeTransform` _returnvalue_location _returnvalue_rotation) "Undefined" "MultiplyWithRoot" null self null))

(fn `DeathAnimation`
  (`SkeletalMeshComponent.PlayAnimation` (`self.Mesh`) "/Game/AI/RangedAssets/Animations/Death.Death" false))

(fn `UserConstructionScript`
  (`parent.UserConstructionScript`))
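; BP_NPC is an enemy pawn that chases and shoots at the player character when its PawnSensing component sees it.
; On sight it turns to face the BP_ThirdPersonCharacter and issues an AI Move To toward it.
; It also spawns a BP_Bullet at a scene component's transform, throttled to one shot per second by a boolean gate and Delay.
; Any damage reduces Health, and the NPC destroys itself at zero.
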(event `self.ReceiveBeginPlay`)

(event `self.ReceiveAnyDamage`
  (params (Damage :type "Float (single-precision)") (DamageType :type "DamageType Object Reference") (InstigatedBy :type "Controller Object Reference") (DamageCauser :type "Actor Object Reference"))
  ;[1 1 1] Any Damage
  (set `self.Health` (- (`self.Health`) Damage))
  (if (<= (`self.Health`) 0.0)
    (`self.K2_DestroyActor`)))

(event `self.PawnSensing.OnSeePawn`
  (params (Pawn :type "Pawn Object Reference"))
  (bind _asbp_third_person_character (cast `/Game/Blueprints/ThirdPerson/Blueprints/BP_ThirdPersonCharacter` Pawn))
  (`|ExecutionSequence`
    (:`then_0`
      (bind _returnvalue (`self.K2_GetActorLocation` _asbp_third_person_character))
      (`self.K2_SetActorRotation` (`KismetMathLibrary.FindLookAtRotation` (`self.K2_GetActorLocation`) _returnvalue))
      (`|AIMoveTo` self _returnvalue _asbp_third_person_character))
    (:`then_1`
      (if (`self.ShootDelay`)
        (`|SpawnActorFromClass` "/Game/AI/AI_Old/BP_Bullet.BP_Bullet_C" (`SceneComponent.K2_GetComponentToWorld` (`self.Scene`)) "Undefined" "MultiplyWithRoot" null null)
        (set `self.ShootDelay` false)
        (`KismetSystemLibrary.Delay` 1.0)
        (set `self.ShootDelay` true)))))

(fn `UserConstructionScript`)
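; BP_Bullet is a projectile actor for ranged AI that damages characters it hits.
; On BeginPlay its sphere component ignores a designated actor while moving.
; On a hit it applies fixed damage to actors tagged Character, then destroys itself on any impact.
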(event `self.ReceiveHit`
  (params (MyComp :type "PrimitiveComponent Object Reference") (Other :type "Actor Object Reference") (OtherComp :type "PrimitiveComponent Object Reference") (bSelfMoved :type Boolean) (HitLocation :type "Vector Structure") (HitNormal :type "Vector Structure") (NormalImpulse :type "Vector Structure") (Hit :type "HitResult Structure (by ref)"))
  (if (`self.ActorHasTag` Other "Character")
    (`GameplayStatics.ApplyDamage` Other 15.0 null self)
    (`self.K2_DestroyActor`)
    (else
      (`self.K2_DestroyActor`))))

(event `self.ReceiveBeginPlay`
  (`PrimitiveComponent.IgnoreActorWhenMoving` (`self.Sphere1`) (`self.IgnoreActor`) true))

(fn `UserConstructionScript`)
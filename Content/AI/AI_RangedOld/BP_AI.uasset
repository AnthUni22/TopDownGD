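; BP_AI is a ranged enemy character that pursues sighted pawns and shoots at the player.
; Pawn sensing triggers AIMoveTo behind a resettable DoOnce, then the capsule turns to the player and spawns a bullet.
; Lethal damage stops movement, plays an animation, adds score to the game instance and destroys it after a delay.
; Death also drops random loot at a nearby reachable point, though RandomInteger(3) never selects the Shotgun option.
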(event `self.ReceiveBeginPlay`
  ;[0 0.2475 1] Set Health
  (`|ExecutionSequence`
    (:`then_0`
      (bind _asbp_third_person_character (cast `/Game/Blueprints/ThirdPerson/Blueprints/BP_ThirdPersonCharacter` (`GameplayStatics.GetPlayerCharacter` 0)))
      (set `self.Player` _asbp_third_person_character)
      (bind _asgame_instance (cast `/Game/UI/LeaderBoard/Game_Instance` (`GameplayStatics.GetGameInstance`)))
      (set `self.As Game Instance` _asgame_instance))
    (:`then_1`
      (set `self.Health` (`self.Health`)))))

(event `self.ReceiveAnyDamage`
  (params (Damage :type "Float (single-precision)") (DamageType :type "DamageType Object Reference") (InstigatedBy :type "Controller Object Reference") (DamageCauser :type "Actor Object Reference"))
  (bind _as_game_instance (`self.As Game Instance`))
  ;[0 0.2475 1] Event Damage AG
  (set `self.Health` (- (`self.Health`) Damage))
  (if (<= (`self.Health`) 0.0)
    (`/Engine/EditorBlueprintResources/StandardMacros.DoOnce` false
      (:`Completed`
        (set `self.dead` true)
        (`self.DisableInput` (`self.GetController`) null)
        (`SkeletalMeshComponent.PlayAnimation` (`self.Mesh`) null false)
        (`CharacterMovementComponent.DisableMovement` (`self.CharacterMovement`))
        (set `/Game/UI/LeaderBoard/Game_Instance.Score` (+ (`/Game/UI/LeaderBoard/Game_Instance.Score` _as_game_instance) (`self.PointsToAdd`)) _as_game_instance)
        (`self.Loot Drop`)
        (`KismetSystemLibrary.Delay` 3.0)
        (`self.K2_DestroyActor`)))))

(event `SeesPawn`
  ;[0 0.2475 1] AI Move To Player Location
  (if (not (`self.dead`))
    (`/Engine/EditorBlueprintResources/StandardMacros.DoOnce` false :!label _label
      (:`Completed`
        (bind _pawn (`self.Pawn`)
          (:`then`
            (`|AIMoveTo` self (`self.K2_GetActorLocation` _pawn) null 300.0
              (:`OnSuccess`
                ;[0 0.2475 1] test bullet hit
                (`SceneComponent.K2_SetWorldRotation` (`self.CapsuleComponent`) (`KismetMathLibrary.FindLookAtRotation` (`self.K2_GetActorLocation`) (`self.K2_GetActorLocation` (`GameplayStatics.GetPlayerCharacter` 0))) false false)
                (`KismetSystemLibrary.Delay` 0.05)
                (`self.Shoot`)
                (`self.LosesPawn`))))
          (:`else`))))))

(event `Shoot`
  (bind (_returnvalue_location _returnvalue_rotation) (`KismetMathLibrary.BreakTransform` (`SceneComponent.K2_GetComponentToWorld` (`self.BulletSpawnPoint`))))
  ;[0 0.2475 1] Shoot / Shoot Delay AG
  (`|SpawnActorFromClass` "/Game/AI/AI_RangedOld/BP_Bullet.BP_Bullet_C" (`KismetMathLibrary.MakeTransform` _returnvalue_location _returnvalue_rotation) "Undefined" "MultiplyWithRoot" null self null))

(event `LosesPawn`
  ;[0 0.2475 1] AI Move To Player Location
  (goto _label :!via `Reset`))

(event `self.PawnSensing.OnSeePawn`
  (params (Pawn :type "Pawn Object Reference"))
  ;[0 0.2475 1] Pawn Sensing AG
  (set `self.Pawn` Pawn)
  (`self.SeesPawn`)
  (`KismetSystemLibrary.RetriggerableDelay` 0.3)
  (`self.LosesPawn`))

(event `Loot Drop`
  (bind _returnvalue (`self.K2_GetActorLocation`))
  ;[0 0.2475 1] Random Loot Drop AG
  (bind _outhit (`KismetSystemLibrary.LineTraceSingle` _returnvalue (- _returnvalue (0.0 0.0 200.0)) "TraceTypeQuery1" false (`|MakeArray` (`GameplayStatics.GetPlayerCharacter` 0) :!type "Actor Object Reference")))
  (`|SpawnActorFromClass` (select `int` (`KismetMathLibrary.RandomInteger` 3) :`0` "/Game/Blueprints/Items/Pickups/BP_AmmoPickUp.BP_AmmoPickUp_C" :`1` "/Game/Blueprints/Items/Pickups/BP_HeathPickUp.BP_HeathPickUp_C" :`2` "/Game/Blueprints/Items/Guns/TestWeapons/AR4.AR4_C" :`3` "/Game/Blueprints/Items/Guns/TestWeapons/Shotgun.Shotgun_C" :!type "Actor Class Reference") (`KismetMathLibrary.MakeTransform` (`NavigationSystemV1.K2_GetRandomReachablePointInRadius` (`.Location` (`GameplayStatics.BreakHitResult` _outhit)) 200.0 null null) (`KismetMathLibrary.MakeRotator` 0.0 0.0 (`KismetMathLibrary.RandomFloatInRange` 0.0 360.0))) "AdjustIfPossibleButDontSpawnIfColliding" "MultiplyWithRoot" null null))

(fn `UserConstructionScript`)
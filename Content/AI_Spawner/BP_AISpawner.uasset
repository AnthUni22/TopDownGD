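; BP_AISpawner is an actor that spawns a limited number of AI enemies at its own location once PortalTrigger fires.
; PortalTrigger starts a looping timer on SpawnEnemy, with a negative initial delay offsetting the first interval.
; Each tick randomly spawns BP_AI or BP_Green with the BT_AI behavior tree and increments a counter.
; When the counter equals NumberOfEnemies, the spawner destroys itself.
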(event `PortalTrigger`
  (`KismetSystemLibrary.K2_SetTimerDelegate` (delegate `SpawnEnemy`) 3.0 true -3.0))

(event `SpawnEnemy`
  (if (== (`self.NumberOfLoops`) (`self.NumberOfEnemies`))
    (`self.K2_DestroyActor`)
    (else
      (`AIBlueprintHelperLibrary.SpawnAIFromClass` (select `int` (`KismetMathLibrary.RandomIntegerInRange` 0 1) :`0` "/Game/AI/AI_New/BP_AI.BP_AI_C" :`1` "/Game/AI/AI_2/BP_Green.BP_Green_C" :!type "Pawn Class Reference") "/Game/AI/AI_New/BT_AI.BT_AI" (`self.K2_GetActorLocation`) (struct) false null)
      (`/Engine/EditorBlueprintResources/StandardMacros.IncrementInt` (`self.NumberOfLoops`)))))

(fn `UserConstructionScript`)
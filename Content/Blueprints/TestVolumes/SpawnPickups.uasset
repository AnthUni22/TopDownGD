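; SpawnPickups is a volume actor that scatters pickup actors inside its Box component when play begins.
; It spawns up to PickupAmount plus one actors, as the loop is inclusive, each at a random point within the box extent.
; A random roll picks the first RandomSpawnActors class about 75% of the time and otherwise the second, since the follow-up roll always passes.
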(event `self.ReceiveBeginPlay`
  (bind _returnvalue (`KismetMathLibrary.RandomIntegerInRange` 1 4))
  (for _ (range (+ (`self.PickupAmount`) 1))
    (if (<= _returnvalue 3)
      (set `self.PickupIndex` 0)
      (`|SpawnActorFromClass` (`|GetArrayItem` (`self.RandomSpawnActors`) (`self.PickupIndex`)) (`KismetMathLibrary.Conv_VectorToTransform` (`KismetMathLibrary.RandomPointInBoundingBox` (`self.K2_GetActorLocation`) (`BoxComponent.BoxExtent` (`self.Box`)))) "Undefined" "MultiplyWithRoot" null null :!label _label)
      (elif (<= _returnvalue 4)
        (set `self.PickupIndex` 1)
        (goto _label)))))

(fn `UserConstructionScript`)
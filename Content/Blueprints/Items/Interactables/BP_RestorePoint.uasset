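; BP_RestorePoint is an interactable restore point that toggles the W_ItemRestorer widget on screen.
; OnInteracted runs a FlipFlop that alternately creates the widget and shows the mouse cursor, or removes the widget and hides the cursor.
; Both branches set Game and UI input mode, so closing does not return to game-only input.
; GetInteractionText supplies a generic "Interact" prompt.
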(event `/Game/UserInterface/BPI_InteractionInterface.OnInteracted`
  (params (Player :type "/Game/Blueprints/ThirdPerson/Blueprints/BP_ThirdPersonCharacter Object Reference"))
  (bind _returnvalue (`GameplayStatics.GetPlayerController` 0))
  (`/Engine/EditorBlueprintResources/StandardMacros.FlipFlop`
    (:`A`
      (bind _returnvalue_2 (`|CreateWidget` "/Game/UI/W_ItemRestorer.W_ItemRestorer_C"))
      (`UserWidget.AddToViewport` _returnvalue_2 0)
      (`WidgetBlueprintLibrary.SetInputMode_GameAndUIEx` _returnvalue null)
      (set `PlayerController.bShowMouseCursor` true _returnvalue))
    (:`B`
      (`Widget.RemoveFromParent` _returnvalue_2)
      (`WidgetBlueprintLibrary.SetInputMode_GameAndUIEx` _returnvalue null)
      (set `PlayerController.bShowMouseCursor` false _returnvalue))))

(fn `GetInteractionText`
  (returns (Text :type Text))
  (return "Interact"))

(fn `UserConstructionScript`
  (`parent.UserConstructionScript`))
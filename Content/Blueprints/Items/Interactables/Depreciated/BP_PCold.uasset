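; BP_PCold is a deprecated PC interactable that toggles a W_PCDialog1 dialog widget on screen.
; A box overlap with BP_ThirdPersonCharacter sets IsOverlapped, which nothing in the graph clears.
; Tick polls whether Tab is held while that flag is set and drives a FlipFlop that alternately creates and removes the widget, so holding Tab toggles it every frame.
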(event `self.Box.OnComponentBeginOverlap`
  (params (OverlappedComponent :type "PrimitiveComponent Object Reference") (OtherActor :type "Actor Object Reference") (OtherComp :type "PrimitiveComponent Object Reference") (OtherBodyIndex :type Integer) (bFromSweep :type Boolean) (SweepResult :type "HitResult Structure (by ref)"))
  (cast `/Game/Blueprints/ThirdPerson/Blueprints/BP_ThirdPersonCharacter` OtherActor)
  (set `self.IsOverlapped?` true))

(event `self.ReceiveTick`
  (params (DeltaSeconds :type "Float (single-precision)"))
  (if (and (`PlayerController.IsInputKeyDown` (`GameplayStatics.GetPlayerController` 0) "Tab") (`self.IsOverlapped?`))
    (`/Engine/EditorBlueprintResources/StandardMacros.FlipFlop`
      (:`A`
        (bind _returnvalue (`|CreateWidget` "/Game/UI/W_PCDialog1.W_PCDialog1_C"))
        (`UserWidget.AddToViewport` _returnvalue 0))
      (:`B`
        (`Widget.RemoveFromParent` _returnvalue)))))

(fn `UserConstructionScript`)
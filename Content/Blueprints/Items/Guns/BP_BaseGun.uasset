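; BP_BaseGun is the base pickup weapon, switching between a physics-simulated Dropped state and a collision-free Equipped state.
; Interacting hands it to the player's PickupGun and equips it.
; Fire spends a magazine round through AttackPattern, a per-gun override that defaults to a BP_Laser with sound, or calls Reload when empty.
; Reload waits out the firing actor's montage, then moves reserve ammo into the magazine.
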(event `self.ReceiveBeginPlay`
  (`self.SetGunState` "NewEnumerator0"))

(event `/Game/UserInterface/BPI_InteractionInterface.OnInteracted`
  (params (Player :type "/Game/Blueprints/ThirdPerson/Blueprints/BP_ThirdPersonCharacter Object Reference"))
  (`/Game/Blueprints/ThirdPerson/Blueprints/BP_ThirdPersonCharacter.PickupGun` Player self)
  (`self.SetGunState` "NewEnumerator1"))

(event `Reload`
  (if (== (`self.CurrentAmmo`) 0)
    _
    (elif (not (`self.Reloading`))
      (set `self.Reloading` true)
      (bind _returnvalue (`AnimInstance.Montage_Play` (`SkeletalMeshComponent.GetAnimInstance` (`Character.Mesh` (`self.FiringActor`))) "/Game/Characters/FutureMan/Animations/ReloadMontage.ReloadMontage" (`self.ReloadRate`) "Duration" 0.0 true))
      (`KismetSystemLibrary.Delay` _returnvalue)
      (set `self.AmmoNeeded` (- (`self.MagSize`) (`self.CurrentMag`)))
      (if (< (`self.CurrentAmmo`) (`self.AmmoNeeded`))
        (set `self.CurrentAmmo` (- (`self.CurrentAmmo`) (`self.CurrentAmmo`)))
        (set `self.CurrentMag` (+ (`self.CurrentMag`) (`self.CurrentAmmo`)))
        (else
          (set `self.CurrentAmmo` (- (`self.CurrentAmmo`) (`self.AmmoNeeded`)))
          (set `self.CurrentMag` (+ (`self.CurrentMag`) (`self.AmmoNeeded`)))))
      (set `self.Reloading` false)
      (set `/Game/Blueprints/ThirdPerson/Blueprints/BP_ThirdPersonCharacter.IsReloading` false (`self.FiringActor`)))))

(fn `AddAmmo`
  (params (AmmoAmount :type Integer))
  (set `self.CurrentAmmo` (+ (`self.CurrentAmmo`) AmmoAmount)))

(fn `AttackPattern`
  (params (InTransform :type "Transform Structure (by ref)"))
  (bind _location (.location InTransform))
  ;[1 1 1] Overide Per Gun
  (`|SpawnActorFromClass` "/Game/Blueprints/BP_Laser.BP_Laser_C" (`KismetMathLibrary.MakeTransform` _location (.rotation InTransform)) "Undefined" "MultiplyWithRoot" null (`self.FiringActor`) null)
  (`GameplayStatics.PlaySoundAtLocation` "/Game/SFX/542579__samsterbirdies__laser.542579__samsterbirdies__laser" _location (struct) 1.0 1.0 0.0 null null null null))

(fn `Drop`
  (`self.SetGunState` "NewEnumerator0"))

(fn `Fire`
  (params (SpawnLocation :type "Transform Structure") (FiringActor :type "/Game/Blueprints/ThirdPerson/Blueprints/BP_ThirdPersonCharacter Object Reference"))
  (bind _output_get (set `self.FiringActor` FiringActor))
  (`/Engine/EditorBlueprintResources/StandardMacros.IsValid` _output_get
    (:`Is Valid`
      (if (== (`self.CurrentMag`) 0)
        (`self.Reload`)
        (else
          (`self.AttackPattern` SpawnLocation)
          (set `self.CurrentMag` (- (`self.CurrentMag`) 1)))))))

(fn `GetInteractionText`
  (returns (Text :type Text))
  (return "Pickup"))

(fn `GetInteractionTextAttach`
  (returns (AttachComponent :type "SceneComponent Object Reference"))
  (return (`self.Gun`)))

(fn `SetGunState`
  (params (NewGunState :type "/Game/Blueprints/Items/Guns/E_GunState Enum" :default "NewEnumerator0"))
  (bind _sphere (`self.Sphere`))
  (bind _gun (`self.Gun`))
  (bind _output_get (set `self.GunState` NewGunState))
  (switch `/Game/Blueprints/Items/Guns/E_GunState` _output_get
    (:`NewEnumerator0`
      (`PrimitiveComponent.SetCollisionProfileName` _sphere "OverlapAllDynamic" true)
      (`PrimitiveComponent.SetSimulatePhysics` _gun true)
      (`PrimitiveComponent.SetCollisionProfileName` _gun "DroppedGun" false))
    (:`NewEnumerator1`
      (`PrimitiveComponent.SetCollisionProfileName` _sphere "NoCollision" true)
      (`PrimitiveComponent.SetSimulatePhysics` _gun false)
      (`PrimitiveComponent.SetCollisionProfileName` _gun "NoCollision" false)
      (`SceneComponent.ResetRelativeTransform` (`self.Gun`)))))

(fn `SetWeaponPerams`
  (params (MaxAmmo :type Integer :default 100) (MagSize :type Integer :default 10) (ReloadRate :type "Float (double-precision)" :default 1.5) (FireRate :type "Float (double-precision)" :default 0.2))
  (bind _output_get (set `self.MaxAmmo` MaxAmmo))
  (set `self.CurrentAmmo` _output_get)
  (bind _output_get_2 (set `self.MagSize` MagSize))
  (set `self.CurrentMag` _output_get_2)
  (set `self.ReloadRate` ReloadRate)
  (set `self.FireRate` FireRate))

(fn `UserConstructionScript`
  (`self.SetWeaponPerams` 100))
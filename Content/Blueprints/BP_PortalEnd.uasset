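; BP_PortalEnd is a level exit portal triggered when BP_ThirdPersonCharacter overlaps its box.
; It spawns a lightning effect, waits briefly, then opens NextWorld if MaxLoopCount is one or less, otherwise increments the character's LevelLoopCount and reloads the current level.
; The branch never reads LevelLoopCount.
; After the open-level call, it increments the Game_Instance Level and stores the primary and secondary gun classes there.
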(event `self.Box.OnComponentBeginOverlap`
  (params (OverlappedComponent :type "PrimitiveComponent Object Reference") (OtherActor :type "Actor Object Reference") (OtherComp :type "PrimitiveComponent Object Reference") (OtherBodyIndex :type Integer) (bFromSweep :type Boolean) (SweepResult :type "HitResult Structure (by ref)"))
  (bind _as_bp_third_person_character (`self.As BP Third Person Character`))
  (bind _asgame_instance (cast `/Game/UI/LeaderBoard/Game_Instance` (`GameplayStatics.GetGameInstance`) :!pure true))
  (bind _asbp_third_person_character (cast `/Game/Blueprints/ThirdPerson/Blueprints/BP_ThirdPersonCharacter` OtherActor))
  (bind _output_get (set `self.As BP Third Person Character` _asbp_third_person_character))
  (`GameplayStatics.SpawnEmitterAtLocation` "/Game/RPGEffects/Particles/P_Mage_Lightning_Shield.P_Mage_Lightning_Shield" (`self.K2_GetActorLocation` _output_get) (struct) (5.0 5.0 5.0))
  (`KismetSystemLibrary.Delay` 2.0)
  (if (>= 0 (- (`self.Max Loop Count`) 1))
    (`GameplayStatics.OpenLevelBySoftObjectPtr` (`self.Next World`))
    (else
      (`/Engine/EditorBlueprintResources/StandardMacros.IncrementInt` (`/Game/Blueprints/ThirdPerson/Blueprints/BP_ThirdPersonCharacter.Level Loop Count` (`self.As BP Third Person Character`))
        (:`  `
          (bind _returnvalue (`GameplayStatics.GetCurrentLevelName` true))
          (`GameplayStatics.OpenLevel` (`KismetStringLibrary.Conv_StringToName` _returnvalue))))))
  (`/Engine/EditorBlueprintResources/StandardMacros.IncrementInt` (`/Game/UI/LeaderBoard/Game_Instance.Level` _asgame_instance)
    (:`  `
      (set `/Game/UI/LeaderBoard/Game_Instance.PrimaryGun` (`GameplayStatics.GetObjectClass` (`/Game/Blueprints/ThirdPerson/Blueprints/BP_ThirdPersonCharacter.PrimaryGun` _as_bp_third_person_character)) _asgame_instance)
      (set `/Game/UI/LeaderBoard/Game_Instance.SecondaryGun` (`GameplayStatics.GetObjectClass` (`/Game/Blueprints/ThirdPerson/Blueprints/BP_ThirdPersonCharacter.SecondaryGun` _as_bp_third_person_character)) _asgame_instance))))

(fn `UserConstructionScript`)
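; BP_BaseGun is a base gun item that lies in the world as an interactable pickup and is equipped by the player who interacts with it.
; It starts Dropped, offers a "Pickup" prompt attached to the Gun component, and on interaction calls the player's PickupGun, then becomes Equipped.
; SetGunState toggles physics and collision on the gun and interaction sphere, resetting the gun's relative transform when equipped.
; Drop restores the Dropped state.
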(event `self.ReceiveBeginPlay`
  (`self.SetGunState` "NewEnumerator0"))

(event `/Game/UserInterface/BPI_InteractionInterface.OnInteracted`
  (params (Player :type "/Game/Blueprints/ThirdPerson/Blueprints/BP_ThirdPersonCharacter Object Reference"))
  (`/Game/Blueprints/ThirdPerson/Blueprints/BP_ThirdPersonCharacter.PickupGun` Player self)
  (`self.SetGunState` "NewEnumerator1"))

(fn `Drop`
  (`self.SetGunState` "NewEnumerator0"))

(fn `GetInteractionText`
  (returns (Text :type Text))
  (return "Pickup"))

(fn `GetInteractionTextAttach`
  (returns (AttachComponent :type "SceneComponent Object Reference"))
  (return (`self.Gun`)))

(fn `SetGunState`
  (params (NewGunState :type "/Game/Items/Guns/E_GunState Enum" :default "NewEnumerator0"))
  (bind _sphere (`self.Sphere`))
  (bind _gun (`self.Gun`))
  (bind _output_get (set `self.GunState` NewGunState))
  (switch `/Game/Items/Guns/E_GunState` _output_get
    (:`NewEnumerator0`
      (`PrimitiveComponent.SetCollisionProfileName` _sphere "OverlapAllDynamic" true)
      (`PrimitiveComponent.SetSimulatePhysics` _gun true)
      (`PrimitiveComponent.SetCollisionProfileName` _gun "DroppedGun" false))
    (:`NewEnumerator1`
      (`PrimitiveComponent.SetCollisionProfileName` _sphere "NoCollision" true)
      (`PrimitiveComponent.SetSimulatePhysics` _gun false)
      (`PrimitiveComponent.SetCollisionProfileName` _gun "NoCollision" false)
      (`SceneComponent.ResetRelativeTransform` (`self.Gun`)))))

(fn `UserConstructionScript`
  (`parent.UserConstructionScript`))
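; Deprecated procedural level cell actor that randomly places walls around itself when play begins.
; BeginPlay rolls a random 0 or 1 per side, spawning a Wall at WallOffset from the cell's location, with west and east walls yawed 90 degrees.
; North, south and east walls depend on their rolls.
; The west wall always spawns because its check is disconnected.
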(event `self.ReceiveBeginPlay`
  (bind _returnvalue (`KismetMathLibrary.RandomInteger` 2))
  (bind _returnvalue_location (`KismetMathLibrary.BreakTransform` (`self.GetTransform`)))
  (bind _returnvalue_location_2 (`KismetMathLibrary.BreakTransform` (`self.GetTransform`)))
  (bind _returnvalue_location_3 (`KismetMathLibrary.BreakTransform` (`self.GetTransform`)))
  (bind _returnvalue_location_4 (`KismetMathLibrary.BreakTransform` (`self.GetTransform`)))
  (bind _output_get (set `self.NorthWall` _returnvalue))
  (`|ExecutionSequence`
    (:`then_0`
      (if (== _output_get 1)
        (`|SpawnActorFromClass` "/Game/ProceduralLevel/DEPRICATED/Blueprints/Wall.Wall_C" (`KismetMathLibrary.MakeTransform` (+ _returnvalue_location (`KismetMathLibrary.MakeVector` 0.0 (`self.WallOffset`)))) "Undefined" "MultiplyWithRoot" null null)))
    (:`then_1`
      (bind _output_get_2 (set `self.SouthWall` _returnvalue))
      (`|ExecutionSequence`
        (:`then_0`
          (if (== _output_get_2 1)
            (`|SpawnActorFromClass` "/Game/ProceduralLevel/DEPRICATED/Blueprints/Wall.Wall_C" (`KismetMathLibrary.MakeTransform` (- _returnvalue_location_2 (`KismetMathLibrary.MakeVector` 0.0 (`self.WallOffset`)))) "Undefined" "MultiplyWithRoot" null null)))
        (:`then_1`
          (bind _output_get_3 (set `self.WestWall` _returnvalue))
          (`|ExecutionSequence`
            (:`then_0`
              (`|SpawnActorFromClass` "/Game/ProceduralLevel/DEPRICATED/Blueprints/Wall.Wall_C" (`KismetMathLibrary.MakeTransform` (+ _returnvalue_location_3 (`KismetMathLibrary.MakeVector` (`self.WallOffset`))) (struct :`Yaw` 90.0)) "Undefined" "MultiplyWithRoot" null null))
            (:`then_1`
              (bind _output_get_4 (set `self.EastWall` _returnvalue))
              (if (== _output_get_4 1)
                (`|SpawnActorFromClass` "/Game/ProceduralLevel/DEPRICATED/Blueprints/Wall.Wall_C" (`KismetMathLibrary.MakeTransform` (- _returnvalue_location_4 (`KismetMathLibrary.MakeVector` (`self.WallOffset`))) (struct :`Yaw` 90.0)) "Undefined" "MultiplyWithRoot" null null)))))))))

(fn `UserConstructionScript`)
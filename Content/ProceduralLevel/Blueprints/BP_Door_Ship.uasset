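; BP_Door_Ship is a two-panel ship door for the procedural level that opens when its OpenDoor event is called.
; A DoOnce that is never reset lets the opening Timeline play only once, with no closing logic.
; Its DoorOpenX and DoorOpenY tracks move both panels in relative space, mirrored on X and together on Y, while each keeps its Z.
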(event `self.OpenDoor`
  (bind _ship_door_l (`self.Ship_Door-L`))
  (bind _ship_door_r (`self.Ship_Door-R`))
  (bind (_relativelocation_x _relativelocation_y _relativelocation_z) (`KismetMathLibrary.BreakVector` (`SceneComponent.RelativeLocation` _ship_door_r)))
  (bind (_relativelocation_x_2 _relativelocation_y_2 _relativelocation_z_2) (`KismetMathLibrary.BreakVector` (`SceneComponent.RelativeLocation` _ship_door_l)))
  (`/Engine/EditorBlueprintResources/StandardMacros.DoOnce` false
    (:`Completed`
      (bind (_direction _dooropen_x _dooropen_y) (`Timeline|Timeline` :!via `PlayFromStart`)
        (:`Update`
          (`SceneComponent.K2_SetRelativeTransform` _ship_door_l (`KismetMathLibrary.MakeTransform` (`KismetMathLibrary.MakeVector` (* _dooropen_x -1.0) _dooropen_y _relativelocation_z_2)) false false)
          (`SceneComponent.K2_SetRelativeTransform` _ship_door_r (`KismetMathLibrary.MakeTransform` (`KismetMathLibrary.MakeVector` _dooropen_x _dooropen_y _relativelocation_z)) false false))))))

(fn `UserConstructionScript`
  (`parent.UserConstructionScript`))
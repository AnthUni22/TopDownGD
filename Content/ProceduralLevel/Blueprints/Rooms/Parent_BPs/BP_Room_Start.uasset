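; BP_Room_Start is the procedural level's start room, which stages the player's arrival through a teleport portal.
; On BeginPlay it hides the third-person character and moves it to the Arrow's location.
; Timelines scale the portal effect up, reveal the player after a short delay, then scale it down by playing in reverse.
; Once the portal closes, it opens every BP_Door overlapping its Sphere.
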(event `self.ReceiveBeginPlay`
  (bind _asbp_third_person_character (cast `/Game/Blueprints/ThirdPerson/Blueprints/BP_ThirdPersonCharacter` (`GameplayStatics.GetPlayerCharacter` 0)))
  (`self.SetActorHiddenInGame` _asbp_third_person_character true)
  (`self.K2_SetActorLocation` _asbp_third_person_character (`SceneComponent.K2_GetComponentLocation` (`self.Arrow`)) false false)
  (`self.Open Portal`))

(event `Open Portal`
  (`SceneComponent.SetHiddenInGame` (`self.P_Status_Teleport_PortalPlayer`) false false)
  (bind (_direction _portal_scale) (`Timeline|Portal Grow` :!via `PlayFromStart`)
    (:`Update`
      (`SceneComponent.SetWorldScale3D` (`self.P_Status_Teleport_PortalPlayer`) (`KismetMathLibrary.Conv_DoubleToVector` _portal_scale)))
    (:`Finished`
      (`self.Teleport Player`))))

(event `Teleport Player`
  (`KismetSystemLibrary.Delay` 0.2)
  (`self.SetActorHiddenInGame` (stale `self.ReceiveBeginPlay` _asbp_third_person_character) false)
  (`KismetSystemLibrary.Delay` 0.2)
  (`self.Close Portal`))

(event `Close Portal`
  (bind (_direction _portal_scale) (`Timeline|Portal Shrink` :!via `ReverseFromEnd`)
    (:`Update`
      (`SceneComponent.SetWorldScale3D` (`self.P_Status_Teleport_PortalPlayer`) (`KismetMathLibrary.Conv_DoubleToVector` _portal_scale)))
    (:`Finished`
      (`SceneComponent.SetHiddenInGame` (`self.P_Status_Teleport_PortalPlayer`) true false)
      (bind _output_get (set `self.Doors` (`PrimitiveComponent.GetOverlappingActors` (`self.Sphere`) "/Game/ProceduralLevel/Blueprints/BP_Door.BP_Door_C")))
      (for _array_element _output_get
        (bind _asbp_door (cast `/Game/ProceduralLevel/Blueprints/BP_Door` _array_element))
        (`/Game/ProceduralLevel/Blueprints/BP_Door.OpenDoor` _asbp_door)))))

(fn `UserConstructionScript`)
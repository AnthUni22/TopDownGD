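; BP_Room is a procedural level room Blueprint that runs an enemy encounter and opens its doors once the room is cleared.
; On BeginPlay it spawns a BP_AISpawner at the Arrow's transform and binds to its room-cleared event.
; The third-person character entering the Box trigger fires the spawner's portal once.
; When cleared, it opens every BP_Door overlapping the Sphere.
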(event `self.ReceiveBeginPlay`
  (bind _returnvalue (`|SpawnActorFromClass` "/Game/AI_Spawner/BP_AISpawner.BP_AISpawner_C" (`SceneComponent.K2_GetComponentToWorld` (`self.Arrow`)) "Undefined" "MultiplyWithRoot" null null))
  (bind _output_get (set `self.Portal` _returnvalue))
  (add `/Game/AI_Spawner/BP_AISpawner.RoomCleared` _output_get (delegate `Open Next Rooms`)))

(event `Open Next Rooms`
  (bind _output_get (set `self.Doors` (`PrimitiveComponent.GetOverlappingActors` (`self.Sphere`) "/Game/ProceduralLevel/Blueprints/BP_Door.BP_Door_C")))
  (for _array_element _output_get
    (bind _asbp_door (cast `/Game/ProceduralLevel/Blueprints/BP_Door` _array_element))
    (`/Game/ProceduralLevel/Blueprints/BP_Door.OpenDoor` _asbp_door)))

(event `self.Box.OnComponentBeginOverlap`
  (params (OverlappedComponent :type "PrimitiveComponent Object Reference") (OtherActor :type "Actor Object Reference") (OtherComp :type "PrimitiveComponent Object Reference") (OtherBodyIndex :type Integer) (bFromSweep :type Boolean) (SweepResult :type "HitResult Structure (by ref)"))
  (cast `/Game/Blueprints/ThirdPerson/Blueprints/BP_ThirdPersonCharacter` OtherActor)
  (`/Engine/EditorBlueprintResources/StandardMacros.DoOnce` false
    (:`Completed`
      (`/Game/AI_Spawner/BP_AISpawner.PortalTrigger` (`self.Portal`)))))

(fn `UserConstructionScript`)
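; Cell actor for a procedural level that can randomly spawn Wall actors around itself.
; Four custom events, one per compass side, each roll a random 0 or 1 and place walls by offsetting the cell's transform; nothing here calls them.
; The south check compares constants, so that wall never spawns.
; West and east walls share the same +X position, differing only in opposite roll offsets.
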(event `CustomEvent`
  (bind _returnvalue (`self.GetTransform`))
  (bind _output_get (set `self.NorthWall` (`KismetMathLibrary.RandomInteger` 2)))
  (if (== _output_get 1)
    (`|SpawnActorFromClass` "/Game/ProceduralLevel/Blueprints/Wall.Wall_C" (`KismetMathLibrary.MakeTransform` (`KismetMathLibrary.MakeVector` (.x (.location _returnvalue)) (+ (.y (.location _returnvalue)) 500.0) (.z (.location _returnvalue)))) "Undefined" "MultiplyWithRoot" null null)))

(event `CustomEvent_1`
  (bind _returnvalue (`self.GetTransform`))
  (set `self.SouthWall` (`KismetMathLibrary.RandomInteger` 2))
  (if (== 0 1)
    (`|SpawnActorFromClass` "/Game/ProceduralLevel/Blueprints/Wall.Wall_C" (`KismetMathLibrary.MakeTransform` (`KismetMathLibrary.MakeVector` (.x (.location _returnvalue)) (+ (.y (.location _returnvalue)) -500.0) (.z (.location _returnvalue)))) "Undefined" "MultiplyWithRoot" null null)))

(event `CustomEvent_2`
  (bind _returnvalue (`self.GetTransform`))
  (bind _output_get (set `self.WestWall` (`KismetMathLibrary.RandomInteger` 2)))
  (if (== _output_get 1)
    (`|SpawnActorFromClass` "/Game/ProceduralLevel/Blueprints/Wall.Wall_C" (`KismetMathLibrary.MakeTransform` (`KismetMathLibrary.MakeVector` (+ (.x (.location _returnvalue)) 500.0) (.y (.location _returnvalue)) (.z (.location _returnvalue))) (`KismetMathLibrary.MakeRotator` (+ (.roll (.rotation _returnvalue)) 90.0) (.pitch (.rotation _returnvalue)) (.yaw (.rotation _returnvalue)))) "Undefined" "MultiplyWithRoot" null null)))

(event `CustomEvent_3`
  (bind _returnvalue (`self.GetTransform`))
  (bind _output_get (set `self.EastWall` (`KismetMathLibrary.RandomInteger` 2)))
  (if (== _output_get 1)
    (`|SpawnActorFromClass` "/Game/ProceduralLevel/Blueprints/Wall.Wall_C" (`KismetMathLibrary.MakeTransform` (`KismetMathLibrary.MakeVector` (+ (.x (.location _returnvalue)) 500.0) (.y (.location _returnvalue)) (.z (.location _returnvalue))) (`KismetMathLibrary.MakeRotator` (+ (.roll (.rotation _returnvalue)) -90.0) (.pitch (.rotation _returnvalue)) (.yaw (.rotation _returnvalue)))) "Undefined" "MultiplyWithRoot" null null)))

(fn `UserConstructionScript`)
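; BP_Door is a double crypt door in the procedural level assets that swings open when the player pawn enters its trigger box.
; The first overlap plays a timeline through a DoOnce, yawing the two leaf meshes in opposite directions; the door never closes again.
; A separate SpawnDoor event spawns another BP_Door at a supplied transform.
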(event `self.Box.OnComponentBeginOverlap`
  (params (OverlappedComponent :type "PrimitiveComponent Object Reference") (OtherActor :type "Actor Object Reference") (OtherComp :type "PrimitiveComponent Object Reference") (OtherBodyIndex :type Integer) (bFromSweep :type Boolean) (SweepResult :type "HitResult Structure (by ref)"))
  (if (== OtherActor (`GameplayStatics.GetPlayerPawn` 0))
    (`/Engine/EditorBlueprintResources/StandardMacros.DoOnce` false
      (:`Completed`
        (bind (_direction _dooropen) (`Timeline|Timeline` :!via `PlayFromStart`)
          (:`Update`
            (`SceneComponent.K2_SetRelativeRotation` (`self.dd1_pasted__polySurface941`) (`KismetMathLibrary.MakeRotator` 0.0 0.0 _dooropen) false false)
            (`SceneComponent.K2_SetRelativeRotation` (`self.dd1_pasted__polySurface940`) (`KismetMathLibrary.MakeRotator` 0.0 0.0 (* _dooropen -1.0)) false false)))))))

(event `SpawnDoor`
  (params (Transform :type "Transform Structure"))
  (`|SpawnActorFromClass` "BP_Door_C" Transform "Undefined" "MultiplyWithRoot" null null))

(fn `UserConstructionScript`)